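; Golf ball character Blueprint with body, arm and leg meshes that also handles level music and dialogue UI.
; Tick sphere-traces downward to place a fake decal shadow on the surface below, hiding it when nothing is hit.
; BeginPlay, outside Intro and Outro, plays music from a start-time offset indexed by the GameInstance's cycling song counter.
; Events spawn dialogue boxes and forward tutorial requests to the first one, while Enter advances waiting dialogue.
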(event EventBeginPlay
  (bind _returnvalue (Game|GetGameInstance))
  (Rendering|SetReceivesDecals (Variables|Default|GetmMesh) false)
  (Rendering|SetReceivesDecals (Variables|Default|GetmLegsMesh) false)
  (Rendering|SetReceivesDecals (Variables|Default|GetmArmsMesh) false)
  (bind _returnvalue_2 (Game|GetCurrentLevelName true))
  (if (Utilities|Enum|NotEqual(Enum) _returnvalue_2 "Intro")
    (if (Utilities|Enum|NotEqual(Enum) _returnvalue_2 "Outro")
      (bind _asgolf_game_instance (Utilities|Casting|CastToGolfGameInstance (Game|GetGameInstance)))
      (Audio|PlaySound2D "/Game/GBH/Sounds/BGMusic_edited_.BGMusic_edited_" (Variables|/Script/Golf04.GolfGameInstance|GetmusicVolume _asgolf_game_instance) 1.0 (Utilities|Array|Get(acopy) (Variables|Default|GetSoundStartTimes) (Variables|/Script/Golf04.GolfGameInstance|GetcurrentSong _asgolf_game_instance)) 0 0)
      (if (>= (Variables|/Script/Golf04.GolfGameInstance|GetcurrentSong _asgolf_game_instance) 5)
        (bind _asgolf_game_instance_2 (Utilities|Casting|CastToGolfGameInstance _returnvalue))
        (Variables|/Script/Golf04.GolfGameInstance|SetcurrentSong _asgolf_game_instance_2 0)
        (else
          (bind _asgolf_game_instance_3 (Utilities|Casting|CastToGolfGameInstance _returnvalue))
          (Math|Integer|IncrementInt (Variables|/Script/Golf04.GolfGameInstance|GetcurrentSong _asgolf_game_instance_3)))))))

(event EventPlayClimbTutorial
  (bind _foundwidgets (Widget|GetAllWidgetsOfClass "/Game/GBH/Widgets/UIWidgets/DialogueBox.DialogueBox_C" true))
  (if (> (Utilities|Array|Length _foundwidgets) 0)
    (Default|PlayClimbTutorial (Utilities|Array|Get(acopy) _foundwidgets))))

(event EventPlayFlyTutorial
  (bind _foundwidgets (Widget|GetAllWidgetsOfClass "/Game/GBH/Widgets/UIWidgets/DialogueBox.DialogueBox_C" true))
  (if (> (Utilities|Array|Length _foundwidgets) 0)
    (Default|PlayFlyingTutorial (Utilities|Array|Get(acopy) _foundwidgets))))

(event EventPrintDialogue
  (params (displayText :type Array%20of%20Strings))
  (bind _returnvalue (UserInterface|CreateWidget "/Game/GBH/Widgets/UIWidgets/DialogueBox.DialogueBox_C" (Game|GetPlayerController 0)))
  (UserInterface|Viewport|AddtoViewport _returnvalue 0)
  (Variables|/Game/GBH/Widgets/UIWidgets/DialogueBox.DialogueBox_C|SetDialogueText _returnvalue displayText)
  (Default|WidgetInitialized _returnvalue))

(event EventTick
  (params (DeltaSeconds :type Float%20%28single-precision%29))
  (bind _shadow (Variables|Default|GetShadow))
  (bind _mmesh (Variables|Default|GetmMesh))
  (bind _returnvalue (Transformation|GetWorldLocation _mmesh))
  (bind (_outhit _returnvalue_2) (Collision|SphereTraceByChannel _returnvalue (+ _returnvalue "0, 0,-2000.000000") 25.0 "TraceTypeQuery1" false 0 "None"))
  (if _returnvalue_2
    (Rendering|SetVisibility _shadow true false)
    (bind _output_get (Variables|Default|SetDecalTargetLocation (.ImpactPoint (Collision|BreakHitResult _outhit))))
    (Transformation|SetWorldLocation _shadow (.Location (Collision|BreakHitResult _outhit)) false false)
    (Transformation|SetWorldRotation _shadow "90.000000, 0, 0" false false)
    (else
      (Rendering|SetVisibility _shadow false false))))

(event EventSwitchDecalVisibility
  (params (visible :type Boolean))
  (Rendering|SetVisibility (Variables|Default|GetShadow) visible false))

(event EventPlayGolfTutorial
  (bind _foundwidgets (Widget|GetAllWidgetsOfClass "/Game/GBH/Widgets/UIWidgets/DialogueBox.DialogueBox_C" true))
  (if (> (Utilities|Array|Length _foundwidgets) 0)
    (Default|PlayGolfTutorial (Utilities|Array|Get(acopy) _foundwidgets))))

(event EventPlayPacmanTutorial
  (bind _foundwidgets (Widget|GetAllWidgetsOfClass "/Game/GBH/Widgets/UIWidgets/DialogueBox.DialogueBox_C" true))
  (if (> (Utilities|Array|Length _foundwidgets) 0)
    (Default|PlayPacmanTutorial (Utilities|Array|Get(acopy) _foundwidgets))))

(event EventPlayWalkTutorial
  (bind _foundwidgets (Widget|GetAllWidgetsOfClass "/Game/GBH/Widgets/UIWidgets/DialogueBox.DialogueBox_C" true))
  (if (> (Utilities|Array|Length _foundwidgets) 0)
    (Default|PlayWalkTutorial (Utilities|Array|Get(acopy) _foundwidgets))))

(event EventPlayZoomTutorial
  (bind _foundwidgets (Widget|GetAllWidgetsOfClass "/Game/GBH/Widgets/UIWidgets/DialogueBox.DialogueBox_C" true))
  (if (> (Utilities|Array|Length _foundwidgets) 0)
    (Default|PlayZoomingTutorial (Utilities|Array|Get(acopy) _foundwidgets))))

(event Input|KeyboardEvents|Enter
  (params (Key :type Key%20Structure))
  (:Pressed
    (bind _foundwidgets (Widget|GetAllWidgetsOfClass "/Game/GBH/Widgets/UIWidgets/DialogueBox.DialogueBox_C" true))
    (if (> (Utilities|Array|Length _foundwidgets) 0)
      (if (Variables|/Game/GBH/Widgets/UIWidgets/DialogueBox.DialogueBox_C|GetbWaitingForInput (Utilities|Array|Get(acopy) _foundwidgets))
        (Default|NextLine (Utilities|Array|Get(acopy) _foundwidgets))))))

(fn ConstructionScript)